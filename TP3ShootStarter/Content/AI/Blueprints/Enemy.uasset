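; Enemy is a shooter AI character that carries a rifle as a child actor snapped to its mesh's weapon socket and forwards start/stop shooting to it.
; Being threatened runs the shoot-from-cover behavior tree and faces the threat, while entering cover crouches and runs the same tree.
; Damage lowers health, and death ragdolls the mesh, stops the AI logic and shooting, and disables capsule collision.
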(event `self.ReceiveBeginPlay`
  (bind _asshooter_enemy_animation (cast `/Game/ImportedContent/ShooterEnemyAnimation` (`SkeletalMeshComponent.GetAnimInstance` (`self.Mesh`))))
  (set `self.AnimInstanse` _asshooter_enemy_animation)
  (bind _asgun_rifle (cast `/Game/ImportedContent/Gun/Gun_Rifle` (`ChildActorComponent.ChildActor` (`self.Gun`))))
  (set `self.CurrentGun` _asgun_rifle))

(event `StartShooting`
  (`/Game/ImportedContent/Gun/Gun_Rifle.StartShooting` (`self.CurrentGun`)))

(event `StopShooting`
  (`/Game/ImportedContent/Gun/Gun_Rifle.StopShooting` (`self.CurrentGun`)))

(event `Threatened`
  (params (ThreatSource :type "Vector Structure"))
  (bind _returnvalue (`AIBlueprintHelperLibrary.GetAIController` self))
  (`AIController.RunBehaviorTree` _returnvalue "/Game/AI/Blueprints/EnemyShootCover.EnemyShootCover")
  (`AIController.K2_SetFocalPoint` _returnvalue ThreatSource))

(event `EnterCover`
  (set `self.IsInCover` true)
  (`self.Crouch`)
  (bind _asenemy_ai (cast `/Game/AI/Blueprints/Enemy_AI` (`AIBlueprintHelperLibrary.GetAIController` null)))
  (`AIController.RunBehaviorTree` _asenemy_ai "/Game/AI/Blueprints/EnemyShootCover.EnemyShootCover"))

(event `self.ReceiveAnyDamage`
  (params (Damage :type "Float (single-precision)") (DamageType :type "DamageType Object Reference") (InstigatedBy :type "Controller Object Reference") (DamageCauser :type "Actor Object Reference"))
  (bind _output_get (set `self.Health` (- (`self.Health`) Damage)))
  (if (<= _output_get 0.0)
    (`PrimitiveComponent.SetSimulatePhysics` (`self.Mesh`) true)
    (`BrainComponent.StopLogic` (`AIController.BrainComponent` (`AIBlueprintHelperLibrary.GetAIController` self)) "")
    (`PrimitiveComponent.SetCollisionEnabled` (`self.CapsuleComponent`) "NoCollision")
    (`self.StopShooting`)
    (else
      (`|PlayMontage` (`self.Mesh`)) ; There is no animation for taking damage so this part is kinda useless
    )))

(fn `UserConstructionScript`
  (`SceneComponent.K2_AttachToComponent` (`self.Gun`) (`self.Mesh`) "Weapon_R" "SnapToTarget" "SnapToTarget" "SnapToTarget" false))