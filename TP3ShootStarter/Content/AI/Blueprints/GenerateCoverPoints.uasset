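; An EQS generator that produces candidate cover points around the first player character for AI queries.
; It casts visibility traces every ten degrees from a ring of the given Radius inward to the player's navmesh-projected location.
; Each hit yields a point offset from the surface along its normal, on the side facing away from the player.
; Points are gathered in LocationSet, then emitted as generated vectors, with brief debug drawing of the traces.
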(fn `DoItemGeneration`
  (params (ContextLocations :type "Array of Vector Structure (by ref)"))
  (bind _projectedlocation (`NavigationSystemV1.K2_ProjectPointToNavigation` (`Actor.K2_GetActorLocation` (`GameplayStatics.GetPlayerCharacter` 0)) null "/Script/NavigationSystem.RecastFilter_UseDefaultArea"))
  (`KismetArrayLibrary.Array_Clear` (`self.LocationSet`))
  (for _index (range 36)
    (bind (_outhit _returnvalue) (`KismetSystemLibrary.LineTraceSingle` :`Start` (+ _projectedlocation (* (`KismetMathLibrary.GreaterGreater_VectorRotator` (1.0 0.0 0.0) (`KismetMathLibrary.MakeRotator` 0.0 0.0 (`KismetMathLibrary.Conv_IntToDouble` (* _index 10)))) (`self.Radius`))) :`End` _projectedlocation :`TraceChannel` "TraceTypeQuery1" :`DrawDebugType` "ForDuration" :`bIgnoreSelf` false :`DrawTime` 0.1))
    (if _returnvalue
      (bind (_bblockinghit _binitialoverlap _time _distance _location _impactpoint _normal _impactnormal) (`GameplayStatics.BreakHitResult` _outhit))
      (`KismetArrayLibrary.Array_Add` (`self.LocationSet`) (+ (* _impactnormal 50.0) _impactpoint))))
  (for _array_element (`self.LocationSet`)
    (`self.AddGeneratedVector` _array_element))
  (return))