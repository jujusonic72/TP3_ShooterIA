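; Enemy_AI is an AI controller that runs the Ennemy_BT behavior tree and caches its controlled Enemy pawn on BeginPlay.
; AI Perception updates for BP_ThirdPersonCharacter write the sensed state to the CanSeePlayer blackboard key.
; When the player is sensed while the enemy is crouching, it also clears IsInCover on the blackboard.
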(event `self.ReceiveBeginPlay`
  (`self.RunBehaviorTree` "/Game/AI/Blueprints/Ennemy_BT.Ennemy_BT")
  (bind _asenemy (cast `/Game/AI/Blueprints/Enemy` (`self.K2_GetPawn`)))
  (set `self.As Enemy` _asenemy))

(event `self.AIPerception.OnTargetPerceptionUpdated`
  (params (Actor :type "Actor Object Reference") (Stimulus :type "AIStimulus Structure"))
  (cast `/Game/ThirdPerson/Blueprints/BP_ThirdPersonCharacter` Actor)
  (bind _output_get (set `self.CanSeePlayer` Stimulus_bSuccessfullySensed))
  (`BlackboardComponent.SetValueAsBool` (`AIBlueprintHelperLibrary.GetBlackboard` null) "CanSeePlayer" _output_get)
  (if (and (`self.CanSeePlayer`) (`NavMovementComponent.IsCrouching` (`Character.CharacterMovement` (`self.As Enemy`))))
    (`BlackboardComponent.SetValueAsBool` (`AIBlueprintHelperLibrary.GetBlackboard` null) "IsInCover" false)))

(fn `UserConstructionScript`)