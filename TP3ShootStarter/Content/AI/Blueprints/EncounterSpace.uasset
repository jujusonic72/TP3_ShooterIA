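; EncounterSpace is an AI encounter volume that shares a target sighting among the Enemy actors inside it.
; Its CalloutTarget event stores the given location, then finds all Enemy actors and keeps those overlapping the space.
; Each of those enemies gets the TargetLocation and a true CanSeePlayer flag written directly into its blackboard, so one callout alerts the group.
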(event `CalloutTarget`
  (params (TargetLocation :type "Vector Structure"))
  (set `self.TargetLocation` TargetLocation)
  (bind _outactors (`GameplayStatics.GetAllActorsOfClass` "/Game/AI/Blueprints/Enemy.Enemy_C"))
  (for _array_element _outactors
    (if (`self.IsOverlappingActor` _array_element)
      (bind _returnvalue (`AIBlueprintHelperLibrary.GetBlackboard` _array_element))
      (`BlackboardComponent.SetValueAsVector` _returnvalue "TargetLocation" (`self.TargetLocation`))
      (`BlackboardComponent.SetValueAsBool` _returnvalue "CanSeePlayer" true))))

(fn `UserConstructionScript`)