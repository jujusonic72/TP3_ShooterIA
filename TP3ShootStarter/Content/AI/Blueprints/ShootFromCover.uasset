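; Behavior tree task that makes an Enemy pop up from cover, shoot for a few seconds and duck back down.
; On execute it uncrouches the pawn, starts shooting and sets a timer that stops fire, crouches and finishes with success.
; Each tick it sets the AI controller's focal point to the player character's location.
; An abort stops shooting and leaves the enemy standing, without clearing the timer.
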(event `self.ReceiveExecuteAI`
  (params (OwnerController :type "AIController Object Reference") (ControlledPawn :type "Pawn Object Reference"))
  (bind _asenemy (cast `/Game/AI/Blueprints/Enemy` ControlledPawn))
  (set `self.EnemyPawn` _asenemy)
  (`Character.UnCrouch` _asenemy)
  (`/Game/AI/Blueprints/Enemy.StartShooting` (`self.EnemyPawn`))
  (`KismetSystemLibrary.K2_SetTimerDelegate` (delegate `StopShooting`) 3.0))

(event `StopShooting`
  (bind _enemypawn (`self.EnemyPawn`))
  (`/Game/AI/Blueprints/Enemy.StopShooting` _enemypawn)
  (`Character.Crouch` _enemypawn)
  (`self.FinishExecute` true))

(event `self.ReceiveTickAI`
  (params (OwnerController :type "AIController Object Reference") (ControlledPawn :type "Pawn Object Reference") (DeltaSeconds :type "Float (single-precision)"))
  (`AIController.K2_SetFocalPoint` OwnerController (`Actor.K2_GetActorLocation` (`GameplayStatics.GetPlayerCharacter` 0))))

(event `self.ReceiveAbortAI`
  (params (OwnerController :type "AIController Object Reference") (ControlledPawn :type "Pawn Object Reference"))
  (bind _enemypawn (`self.EnemyPawn`))
  (`Character.UnCrouch` _enemypawn)
  (`/Game/AI/Blueprints/Enemy.StopShooting` _enemypawn)
  (`self.FinishAbort`))